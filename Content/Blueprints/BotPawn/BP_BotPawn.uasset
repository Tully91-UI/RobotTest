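; BP_BotPawn is a player-controlled flying bot pawn that shoots energy beams from two rifle sockets.
; BeginPlay adds the Enhanced Input context, feeding look input to controller yaw and pitch and three-axis move input along control-rotation axes into FloatingPawnMovement.
; Tick snaps the bot mesh to the control rotation.
; Fire alternates left and right muzzles via FlipFlop, spawning a beam actor, Niagara burst and sound at that socket.
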(event `self.ReceiveBeginPlay`
  (`self.AddInputMappingContext`))

(event `EnhancedInput|/Game/Blueprints/Input/InputActions/IA_Fire`
  (params (ActionValue :type Boolean) (ElapsedSeconds :type "Float (double-precision)") (TriggeredSeconds :type "Float (double-precision)") (InputAction :type "InputAction Object Reference" :default "/Game/Blueprints/Input/InputActions/IA_Fire.IA_Fire"))
  (:`Started`
    (`/Engine/EditorBlueprintResources/StandardMacros.FlipFlop`
      (:`A`
        (`self.SpawnBeam` "Rifle_L"))
      (:`B`
        (`self.SpawnBeam` "Rifle_R")))))

(event `EnhancedInput|/Game/Blueprints/Input/InputActions/IA_Look`
  (params (ActionValue :type "Vector2D Structure") (ElapsedSeconds :type "Float (double-precision)") (TriggeredSeconds :type "Float (double-precision)") (InputAction :type "InputAction Object Reference" :default "/Game/Blueprints/Input/InputActions/IA_Look.IA_Look"))
  (:`Triggered`
    (`self.HandleLookInput` ActionValue)))

(event `EnhancedInput|/Game/Blueprints/Input/InputActions/IA_Move`
  (params (ActionValue :type "Vector Structure") (ElapsedSeconds :type "Float (double-precision)") (TriggeredSeconds :type "Float (double-precision)") (InputAction :type "InputAction Object Reference" :default "/Game/Blueprints/Input/InputActions/IA_Move.IA_Move"))
  (:`Triggered`
    (`self.HandleFloatingPawnMovement`)))

(event `self.ReceiveTick`
  (params (DeltaSeconds :type "Float (single-precision)"))
  (`self.RotateMeshToController`))

(fn `AddInputMappingContext`
  (bind _asplayer_controller (cast `PlayerController` (`self.GetController`)))
  (`EnhancedInputSubsystemInterface.AddMappingContext` (pcsubsystem `EnhancedInputLocalPlayerSubsystem` _asplayer_controller) "/Game/Blueprints/Input/IMC_Bot.IMC_Bot" 0 (struct)))

(fn `GetForwardInputVector`
  (returns (ReturnValue :type "Vector Structure"))
  (bind (_returnvalue_x _returnvalue_y) (`KismetMathLibrary.BreakVector` (`|GetInputActionValue`)))
  (return (* (`KismetMathLibrary.GetForwardVector` (`self.GetControlRotation`)) _returnvalue_y)))

(fn `GetRightInputVector`
  (returns (ReturnValue :type "Vector Structure"))
  (bind _returnvalue_x (`KismetMathLibrary.BreakVector` (`|GetInputActionValue`)))
  (return (* (`KismetMathLibrary.GetRightVector` (`self.GetControlRotation`)) _returnvalue_x)))

(fn `GetUpInputVector`
  (returns (ReturnValue :type "Vector Structure"))
  (bind (_returnvalue_x _returnvalue_y _returnvalue_z) (`KismetMathLibrary.BreakVector` (`|GetInputActionValue`)))
  (return (* (`KismetMathLibrary.GetUpVector` (`self.GetControlRotation`)) _returnvalue_z)))

(fn `HandleFloatingPawnMovement`
  (bind _floatingpawnmovement (`self.FloatingPawnMovement`))
  (`PawnMovementComponent.AddInputVector` _floatingpawnmovement (`self.GetRightInputVector`) false)
  (`PawnMovementComponent.AddInputVector` _floatingpawnmovement (`self.GetForwardInputVector`) false)
  (`PawnMovementComponent.AddInputVector` _floatingpawnmovement (`self.GetUpInputVector`) false))

(fn `HandleLookInput`
  (params (InVec :type "Vector2D Structure"))
  (bind (_x _y) (`KismetMathLibrary.BreakVector2D` InVec))
  (`self.AddControllerYawInput` _x)
  (`self.AddControllerPitchInput` _y))

(fn `RotateMeshToController`
  (`SceneComponent.K2_SetWorldRotation` (`self.BotMesh`) (`self.GetControlRotation`) false false))

(fn `SpawnBeam`
  (params (`Socket Name` :type Name))
  (bind _returnvalue (`SceneComponent.GetSocketTransform` (`self.BotMesh`) `Socket Name` "RTS_World"))
  (bind _location (.location _returnvalue))
  (`|SpawnActorFromClass` "/Game/Blueprints/Beam/BP_PlayerBeam.BP_PlayerBeam_C" _returnvalue "Undefined" "MultiplyWithRoot" null null null)
  (`NiagaraFunctionLibrary.SpawnSystemAtLocation` "/Game/Assets/FX/NS_BeamBurst.NS_BeamBurst" _location (.rotation _returnvalue))
  (`GameplayStatics.PlaySoundAtLocation` "/Game/Assets/Sounds/Drone/SFX_EnergyRifle.SFX_EnergyRifle" _location (struct) 1.0 1.0 0.0 null null null null))

(fn `UserConstructionScript`)