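; Small sphere pickup that drifts through the level and increments the BP_RobotGameMode score when a Pawn overlaps it.
; On spawn it scales in via timeline, picks a random spin rate and starts a lifetime timer.
; Tick moves it along the mesh's forward vector while spinning the actor, so its heading keeps changing.
; Overlap triggers a guarded fade-out timeline that animates scale, then destroys the actor.
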(event `self.ReceiveBeginPlay`
  (`self.FadeIn`)
  (`self.InitializeDeltaRotation`)
  ;[0 0.15 0.04244 0.5] Start fade in timeline
  (`KismetSystemLibrary.K2_SetTimerDelegate` (`|CreateDelegate` :!event `FadeOut`) (`self.Lifetime`))
  (add `PrimitiveComponent.OnComponentBeginOverlap` (`self.SphereVolume`) (`|CreateDelegate` :!event `OnSphereOverlap`)))

(event `self.ReceiveTick`
  (params (DeltaSeconds :type "Float (single-precision)"))
  ;[0 0.15 0.04244 0.5] Update movement properties of sphere
  (`self.UpdateLocation` DeltaSeconds)
  (`self.UpdateRotation` DeltaSeconds))

(event `FadeIn`
  ;[0 0.15 0.04244 0.5] Fade in when spawning
  (bind (_direction _scale) (`Timeline|FadeInTimeline`)
    (:`Update`
      (`SceneComponent.SetWorldScale3D` (`self.SphereMesh`) _scale))))

(event `FadeOut`
  ;[0 0.15 0.04244 0.5] Fade out to destroy
  (if (not (`self.IsFading`))
    (set `self.IsFading` true)
    (bind (_direction _scale) (`Timeline|FadeOutTimeline`)
      (:`Update`
        (`self.UpdateScale` _scale))
      (:`Finished`
        (`self.K2_DestroyActor`)))))

(event `OnSphereOverlap`
  (params (OverlappedComponent :type "PrimitiveComponent Object Reference") (OtherActor :type "Actor Object Reference") (OtherComp :type "PrimitiveComponent Object Reference") (OtherBodyIndex :type Integer) (bFromSweep :type Boolean) (SweepResult :type "HitResult Structure (by ref)"))
  (if (`GameplayStatics.ObjectIsA` OtherActor "/Script/Engine.Pawn")
    (bind _asbp_robot_game_mode (cast `/Game/Blueprints/Game/BP_RobotGameMode` (`GameplayStatics.GetGameMode`)))
    (`/Game/Blueprints/Game/BP_RobotGameMode.IncrementScore` _asbp_robot_game_mode)
    (`self.FadeOut`)))

(fn `InitializeDeltaRotation`
  (set `self.DeltaRotation` (* (`KismetMathLibrary.RandomRotator` false) (`self.RotationScaleFactor`))))

(fn `UpdateLocation`
  (params (`Delta Time` :type "Float (double-precision)"))
  (`self.K2_AddActorWorldOffset` (* (`SceneComponent.GetForwardVector` (`self.SphereMesh`)) (* (`self.Speed`) (`local.Delta Time`)))))

(fn `UpdateRotation`
  (params (`Delta Time` :type "Float (double-precision)"))
  (`self.K2_AddActorWorldRotation` (* (`self.DeltaRotation`) (`local.Delta Time`))))

(fn `UpdateScale`
  (params (Scale :type "Float (single-precision)"))
  (`SceneComponent.SetWorldScale3D` (`self.SphereMesh`) (`KismetMathLibrary.MakeVector` Scale Scale Scale)))

(fn `UserConstructionScript`)