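; BP_SphereSpawner is an actor that keeps spawning BP_SmallSphere actors around itself.
; On BeginPlay it starts a looping timer at the SpawnTimer interval to drive sphere spawning.
; Each spawn gets a random rotation and a location found by pushing a random direction out by a random distance up to SpawnRadius from the spawner.
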(event `self.ReceiveBeginPlay`
  ;[0 0.15 0.04244 0.5] Setup sphere spawning timer
  (`KismetSystemLibrary.K2_SetTimerDelegate` (`|CreateDelegate` :!event `SpawnSphere`) (`self.SpawnTimer`) true))

(event `SpawnSphere`
  (`self.HandleSphereSpawning`))

(fn `GetRandomLocationInRadius`
  (returns (RandomLocation :type "Vector Structure"))
  (return (+ (* (`KismetMathLibrary.GetForwardVector` (`KismetMathLibrary.RandomRotator` false)) (`KismetMathLibrary.RandomFloatInRange` 0.0 (`self.SpawnRadius`))) (`self.K2_GetActorLocation`))))

(fn `HandleSphereSpawning`
  (`|SpawnActorFromClass` "/Game/Blueprints/SmallSphere/BP_SmallSphere.BP_SmallSphere_C" (`KismetMathLibrary.MakeTransform` (`self.GetRandomLocationInRadius`) (`KismetMathLibrary.RandomRotator` false)) "Undefined" "MultiplyWithRoot" null null))

(fn `UserConstructionScript`)